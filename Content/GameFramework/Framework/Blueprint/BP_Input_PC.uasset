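; Player controller Blueprint that detects whether desktop input comes from keyboard/mouse or another device, such as a gamepad.
; On Windows, Mac and Linux, each key press is classified and acted on only when the input type changes.
; A change updates the IsComputer flag and mouse cursor visibility.
; It then fetches the HUD's widget input stack and tells each entry to refresh its input icons through interface messages.
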(event `Key|AnyKey` :consume false :overrideparent false
  (params (Key :type "Key Structure"))
  (bind _key (`self.Key`))
  (bind _returnvalue (or (`KismetInputLibrary.Key_IsKeyboardKey` _key) (`KismetInputLibrary.Key_IsMouseButton` _key)))
  (:`Pressed`
    (set `self.Key` Key)
    (switch `string` (`GameplayStatics.GetPlatformName`)
      (:`Windows`
        _)
      (:`Mac`
        _)
      (:`Linux`
        _))
    (if (!= (`self.IsComputer`) _returnvalue)
      (bind _output_get (set `self.IsComputer` _returnvalue)) ; Only set on update
      (set `self.bShowMouseCursor` _output_get)
      (bind _widgets (message `/Game/GameFramework/Framework/Blueprint/BPI_HUDInput.BPI_GetWidgetInputStack` (`self.GetHUD`)))
      (for _array_element _widgets
        (message `/Game/GameFramework/Framework/UI/Blueprint/BPI_WidgetInput.BPI_UpdateInputIcons` _array_element)))))

(fn `UserConstructionScript`)