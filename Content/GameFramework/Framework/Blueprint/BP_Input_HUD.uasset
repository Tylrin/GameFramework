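; BP_Input_HUD is a HUD Blueprint that keeps a stack of widgets for input handling.
; Its BPI-prefixed functions add a widget uniquely, remove a given widget, or return the whole WidgetInputStack array.
; The current input item is the array's last element, fetched without an empty check.
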(fn `BPI_AddItemToWidgetStack`
  (params (Widget :type "/Game/GameFramework/Framework/UI/Widgets/Components/WidgetWindow Object Reference"))
  (returns (Index :type Integer))
  (bind _returnvalue (`KismetArrayLibrary.Array_AddUnique` (`self.WidgetInputStack`) Widget))
  (return _returnvalue))

(fn `BPI_GetWidgetInputItem`
  (returns (Widget :type "/Game/GameFramework/Framework/UI/Widgets/Components/WidgetWindow Object Reference"))
  (bind _widgetinputstack (`self.WidgetInputStack`))
  (return (`|GetArrayItem` _widgetinputstack (`KismetArrayLibrary.Array_LastIndex` _widgetinputstack))))

(fn `BPI_GetWidgetInputStack`
  (returns (Widgets :type "Array of /Game/GameFramework/Framework/UI/Widgets/Components/WidgetWindow Object Reference"))
  (return (`self.WidgetInputStack`)))

(fn `BPI_RemoveItemFromWidgetStack`
  (params (Widget :type "/Game/GameFramework/Framework/UI/Widgets/Components/WidgetWindow Object Reference"))
  (returns (RetrunValue :type Boolean))
  (bind _returnvalue (`KismetArrayLibrary.Array_RemoveItem` (`self.WidgetInputStack`) Widget))
  (return _returnvalue))

(fn `UserConstructionScript`)