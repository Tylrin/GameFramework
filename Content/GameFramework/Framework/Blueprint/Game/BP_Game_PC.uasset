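; BP_Game_PC is the in-game player controller that handles pause input.
; On BeginPlay it adds the pause-menu Enhanced Input mapping context and sets game-only input, then removes the context when destroyed.
; The pause action asks BP_Game_HUD to show the pause menu.
; A hardwired E key press loads MenuLevel directly, bypassing the input action system.
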(event `self.ReceiveBeginPlay`
  ;[0.1529 0.7529 0.2099] Event Begin Play
  (`EnhancedInputSubsystemInterface.AddMappingContext` (subsystem `EnhancedInputLocalPlayerSubsystem`) "/Game/GameFramework/Framework/Input/IM_PauseMenuControls_InputMapping.IM_PauseMenuControls_InputMapping" 0)
  (`WidgetBlueprintLibrary.SetInputMode_GameOnly` self))

(event `self.ReceiveDestroyed`
  ;[0 0 0 0.5] Event Destroyed
  (`EnhancedInputSubsystemInterface.RemoveMappingContext` (subsystem `EnhancedInputLocalPlayerSubsystem`) "/Game/GameFramework/Framework/Input/IM_PauseMenuControls_InputMapping.IM_PauseMenuControls_InputMapping"))

(event `EnhancedInput|/Game/GameFramework/Framework/Input/IA_Pause`
  (params (ActionValue :type Boolean) (ElapsedSeconds :type "Float (single-precision)") (TriggeredSeconds :type "Float (single-precision)"))
  ;[0 0 0 0.5] Pause
  (:`Started`
    (bind _asbp_game_hud (cast `/Game/GameFramework/Framework/Blueprint/Game/BP_Game_HUD` (`self.GetHUD`)))
    (`/Game/GameFramework/Framework/Blueprint/Game/BP_Game_HUD.Event_ShowPauseMenu` _asbp_game_hud)))

(event `Key|E`
  (params (Key :type "Key Structure"))
  (:`Pressed`
    (`GameplayStatics.OpenLevel` "MenuLevel")))

(fn `UserConstructionScript`)