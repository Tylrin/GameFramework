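; BP_Game_HUD is the game HUD that opens the pause menu and manages input mode and mouse cursor around it.
; Showing the menu removes any existing widget, creates a new UI_PauseMenu and binds to its window-close event.
; It uses Game and UI input so input actions keep working while the menu is open.
; The window-closed handler restores game-only input and hides the cursor.
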(event `Event_ShowPauseMenu`
  (bind _returnvalue (`self.GetOwningPlayerController`))
  (bind _menuwidget (`self.MenuWidget`))
  ;[0 0 0 0.5] Event Show Pause Menu
  (`/Engine/EditorBlueprintResources/StandardMacros.IsValid` _menuwidget
    (:`Is Valid`
      (`Widget.RemoveFromParent` _menuwidget))
    (:`Is Not Valid`
      _))
  (bind _returnvalue_2 (`|CreateWidget` "/Game/GameFramework/Framework/UI/Widgets/Gameplay/UI_PauseMenu.UI_PauseMenu_C" (`self.GetOwningPlayerController`)))
  (bind _output_get (set `self.MenuWidget` _returnvalue_2))
  (`UserWidget.AddToViewport` _output_get 0)
  (add `/Game/GameFramework/Framework/UI/Widgets/Components/WidgetWindow.OnWindowClose` _output_get (`|CreateDelegate` :!event `Event_OnWindowClosed`))
  (`WidgetBlueprintLibrary.SetInputMode_GameAndUIEx` _returnvalue (`self.MenuWidget`) "DoNotLock" false) ; Use Game and UI so that the Input Actions still works.
  (set `PlayerController.bShowMouseCursor` true _returnvalue))

(event `Event_OnWindowClosed`
  (bind _returnvalue (`self.GetOwningPlayerController`))
  ;[0 0 0] Event On Window Closed
  (`WidgetBlueprintLibrary.SetInputMode_GameOnly` _returnvalue)
  (set `PlayerController.bShowMouseCursor` false _returnvalue))

(fn `UserConstructionScript`
  (`parent.UserConstructionScript`))