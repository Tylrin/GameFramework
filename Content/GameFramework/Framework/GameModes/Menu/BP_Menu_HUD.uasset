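; Menu HUD that puts either the startup menu or the main menu layout on screen when play begins.
; BeginPlay reads the StartOption from the game mode's options string and shows the main menu when requested, defaulting to the start menu.
; Each show event replaces the current menu widget and focuses the new one in Game and UI input mode so Input Actions keep working.
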(event `self.ReceiveBeginPlay`
  ;[0.1529 0.7529 0.2099] Event Begin Play
  (switch `string` (`GameplayStatics.ParseOption` (`GameModeBase.OptionsString` (`GameplayStatics.GetGameMode`)) "StartOption")
    (:`Default`
      (`self.Event_ShowStartMenu` :!label _label))
    (:`MainMenu`
      (`self.Event_ShowMainMenu`))
    (:`StartMenu`
      (goto _label))))

(event `Event_ShowStartMenu`
  (bind _menuwidget (`self.MenuWidget`))
  ;[0 0 0 0.5] Event Show Start Menu
  (`/Engine/EditorBlueprintResources/StandardMacros.IsValid` _menuwidget
    (:`Is Valid`
      (`Widget.RemoveFromParent` _menuwidget))
    (:`Is Not Valid`
      _))
  (bind _returnvalue (`|CreateWidget` "/Game/GameFramework/Framework/UI/Widgets/UI_StartupMenuLayout_Persistant.UI_StartupMenuLayout_Persistant_C" (`GameplayStatics.GetPlayerController` 0)))
  (bind _output_get (set `self.MenuWidget` _returnvalue))
  (`UserWidget.AddToViewport` _output_get 0)
  (`WidgetBlueprintLibrary.SetInputMode_GameAndUIEx` (`GameplayStatics.GetPlayerController` 0) (`self.MenuWidget`) "DoNotLock" false) ; Use Game and UI so that the Input Actions still works.
)

(event `Event_ShowMainMenu`
  (bind _menuwidget (`self.MenuWidget`))
  ;[0 0 0 0.5] Event Show Main Menu
  (`/Engine/EditorBlueprintResources/StandardMacros.IsValid` _menuwidget
    (:`Is Valid`
      (`Widget.RemoveFromParent` _menuwidget))
    (:`Is Not Valid`
      _))
  (bind _returnvalue (`|CreateWidget` "/Game/GameFramework/Framework/UI/Widgets/UI_MainMenuLayout_Persistant.UI_MainMenuLayout_Persistant_C" (`GameplayStatics.GetPlayerController` 0)))
  (bind _output_get (set `self.MenuWidget` _returnvalue))
  (`UserWidget.AddToViewport` _output_get 0)
  (`WidgetBlueprintLibrary.SetInputMode_GameAndUIEx` (`GameplayStatics.GetPlayerController` 0) (`self.MenuWidget`) "DoNotLock" false) ; Use Game and UI so that the Input Actions still works.
)

(fn `UserConstructionScript`)