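; Menu player controller that switches Enhanced Input mapping contexts between the start screen and the main menu.
; On BeginPlay it reads the StartOption game mode option to add either the start menu or general menu mapping, defaulting to the latter.
; The Start action tells BP_Menu_HUD to show the main menu, then swaps mappings.
; Destroyed removes both contexts, while Confirm and Cancel actions are empty stubs.
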(event `self.ReceiveBeginPlay`
  (bind _returnvalue (subsystem `EnhancedInputLocalPlayerSubsystem`))
  ;[0.1529 0.7529 0.2099] Event BeginPlay
  (switch `string` (`GameplayStatics.ParseOption` (`GameModeBase.OptionsString` (`GameplayStatics.GetGameMode`)) "StartOption")
    (:`Default`
      (`EnhancedInputSubsystemInterface.AddMappingContext` _returnvalue "/Game/GameFramework/Framework/Input/IM_MenuControls_InputMapping.IM_MenuControls_InputMapping" 0 :!label _label))
    (:`StartMenu`
      (`EnhancedInputSubsystemInterface.AddMappingContext` _returnvalue "/Game/GameFramework/Framework/Input/IM_StartMenuControls_InputMapping.IM_StartMenuControls_InputMapping" 0))
    (:`MainMenu`
      (goto _label))))

(event `self.ReceiveDestroyed`
  (bind _returnvalue (subsystem `EnhancedInputLocalPlayerSubsystem`))
  ;[0 0 0 0.5] Event Destroyed
  (`EnhancedInputSubsystemInterface.RemoveMappingContext` _returnvalue "/Game/GameFramework/Framework/Input/IM_StartMenuControls_InputMapping.IM_StartMenuControls_InputMapping")
  (`EnhancedInputSubsystemInterface.RemoveMappingContext` _returnvalue "/Game/GameFramework/Framework/Input/IM_MenuControls_InputMapping.IM_MenuControls_InputMapping"))

(event `EnhancedInput|/Game/GameFramework/Framework/Input/IA_Start`
  (params (ActionValue :type Boolean) (ElapsedSeconds :type "Float (single-precision)") (TriggeredSeconds :type "Float (single-precision)"))
  (bind _returnvalue (subsystem `EnhancedInputLocalPlayerSubsystem`))
  ;[0 0 0 0.5] Input Action // Press Start
  (:`Started`
    (bind _asbp_menu_hud (cast `/Game/GameFramework/Framework/GameModes/Menu/BP_Menu_HUD` (`self.GetHUD`)))
    (`/Game/GameFramework/Framework/GameModes/Menu/BP_Menu_HUD.Event_ShowMainMenu` _asbp_menu_hud)
    (`EnhancedInputSubsystemInterface.RemoveMappingContext` _returnvalue "/Game/GameFramework/Framework/Input/IM_StartMenuControls_InputMapping.IM_StartMenuControls_InputMapping")
    (`EnhancedInputSubsystemInterface.AddMappingContext` _returnvalue "/Game/GameFramework/Framework/Input/IM_MenuControls_InputMapping.IM_MenuControls_InputMapping" 0)))

(event `EnhancedInput|/Game/GameFramework/Framework/Input/IA_Confirm`
  (params (ActionValue :type Boolean) (ElapsedSeconds :type "Float (single-precision)") (TriggeredSeconds :type "Float (single-precision)"))
  ;[0 0 0 0.5] Input Action // Confirm
)

(event `EnhancedInput|/Game/GameFramework/Framework/Input/IA_Cancel`
  (params (ActionValue :type Boolean) (ElapsedSeconds :type "Float (single-precision)") (TriggeredSeconds :type "Float (single-precision)"))
  ;[0 0 0 0.5] Input Action // Cancel
)

(fn `UserConstructionScript`)