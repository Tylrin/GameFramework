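; BP_BaseGameSave keeps the list of save game slot names, with functions to add, remove and return them.
; Adding appends a "SaveGame_" name numbered by the current list length, so names can repeat after a removal.
; The OnSaveGameListChanged dispatcher fires after each add and each successful removal.
; These functions only edit the list and do not write or delete saves on disk.
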(fn `AddSaveGameSlot`
  ;[0 0 0] Add Save Game Slot
  (`KismetArrayLibrary.Array_Add` (`self.SaveGameSlots`) (`KismetStringLibrary.Concat_StrStr` "SaveGame_" (`KismetStringLibrary.Conv_IntToString` (+ (`KismetArrayLibrary.Array_LastIndex` (`self.SaveGameSlots`)) 1))))
  (`self.OnSaveGameListChanged`))

(fn `GetSaveGameSlots`
  (returns (SaveGameSlots :type "Array of String"))
  (return (`self.SaveGameSlots`)))

(fn `RemoveSaveGameSlot`
  (params (Item :type "String (by ref)"))
  (returns (ReturnValue :type Boolean))
  ;[0 0 0] Remove Save Game Slot
  (bind _returnvalue (`KismetArrayLibrary.Array_RemoveItem` (`self.SaveGameSlots`) Item))
  (if _returnvalue
    (`self.OnSaveGameListChanged`))
  (return _returnvalue))